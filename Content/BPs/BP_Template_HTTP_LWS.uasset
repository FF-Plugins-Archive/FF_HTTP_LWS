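; Template Blueprint that starts an HTTP server from the FF_HTTP_LWS plugin and answers incoming requests.
; On BeginPlay it resolves the plugin's Resources/wwwroot folder, spawns an HTTP_Server_LWS actor with that root and binds a message event.
; Each request prints its URI and sends a response without setting header entries.
; Body and User-Agent getters exist but are unwired, so their printed labels stay empty.
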(event `self.ReceiveBeginPlay`
  (bind (_outbasedir _returnvalue) (`PluginBlueprintLibrary.GetPluginBaseDir` "FF_HTTP_LWS"))
  (if _returnvalue
    (set `self.Path_Root` (`KismetSystemLibrary.ConvertToAbsolutePath` (`KismetStringLibrary.Concat_StrStr` _outbasedir "/Resources/wwwroot"))))
  (bind _returnvalue_2 (`|SpawnActorFromClass` "/Script/FF_HTTP_LWS.HTTP_Server_LWS" (`KismetMathLibrary.MakeTransform` (0.0 0.0 0.0)) "Undefined" "MultiplyWithRoot" null (`self.Path_Root`) "404.html" 8081 8453 "api/lws/v1/" "LibWebSocket" null))
  (add `HTTP_Server_LWS.DelegateHttpMessageAdv` _returnvalue_2 (delegate `CustomEvent`)))

(event `CustomEvent`
  (params (Connection :type "HttpConnectionLws Object Reference"))
  (`KismetSystemLibrary.PrintString` (`KismetStringLibrary.Concat_StrStr` "Uri = " (`HttpConnectionLws.GetUri` Connection) " \n" "Body = " "" " \n" "Header = ") true true (struct :`G` 0.66 :`B` 1.0 :`A` 1.0) 30.0)
  (`HttpConnectionLws.SendResponse` Connection "" (`|MakeMap`) true 200))

(fn `UserConstructionScript`)